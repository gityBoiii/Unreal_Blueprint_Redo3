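; BP_DefaultPawn is a pawn that lets the player shoot and destroy targets with the left mouse button.
; On click it runs a Visibility line trace forward from the camera, with debug drawing.
; A hit NewBlueprint actor is destroyed, with a smoke emitter at the impact point and a 2D explosion sound.
; Print strings report the explosion steps or a non-matching hit; BeginPlay, overlap and Tick are empty.
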(event `Key|LeftMouseButton`
  (params (Key :type "Key Structure"))
  (bind _returnvalue (`GameplayStatics.GetPlayerCameraManager` 0))
  (bind _returnvalue_2 (`PlayerCameraManager.GetCameraLocation` _returnvalue))
  (:`Pressed`
    (bind (_outhit _returnvalue_3) (`KismetSystemLibrary.LineTraceSingle` :`Start` _returnvalue_2 :`End` (+ _returnvalue_2 (* (`KismetMathLibrary.GetForwardVector` (`PlayerCameraManager.GetCameraRotation` _returnvalue)) 10000.0)) :`TraceChannel` "TraceTypeQuery1" :`DrawDebugType` "ForDuration"))
    (if _returnvalue_3
      (bind (_bblockinghit _binitialoverlap _time _distance _location _impactpoint _normal _impactnormal _physmat _hitactor) (`GameplayStatics.BreakHitResult` _outhit))
      (cast `/Game/Blueprints/NewBlueprint` _hitactor
        (:`then`
          (`self.K2_DestroyActor` _hitactor)
          (`KismetSystemLibrary.PrintString` "폭발 전")
          ;[1 1 1] 폭발
          (`GameplayStatics.SpawnEmitterAtLocation` "/Game/StarterContent/Particles/P_Smoke.P_Smoke" _location)
          (`KismetSystemLibrary.PrintString` "폭발 후")
          (`GameplayStatics.PlaySound2D` "/Game/StarterContent/Audio/Explosion_Cue.Explosion_Cue" 1.0 1.0 0.0 null null))
        (:`CastFailed`
          (`KismetSystemLibrary.PrintString` "NewBlueprint 아님!"))))))

(fn `UserConstructionScript`)